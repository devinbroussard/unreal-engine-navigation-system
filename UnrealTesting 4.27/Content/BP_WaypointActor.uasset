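; Waypoint actor that registers a colored marker with the player's navigation HUD.
; On its first successful Tick it builds a waypoint from the player character's transform, not its own, and its color, then adds it to the HUD's waypoint list.
; A flag stops repeat additions, and Tick retries until the ThirdPersonCharacter cast succeeds.
; EndPlay removes the stored waypoint from that list.
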(event EventTick
  (params (DeltaSeconds :type Float%20%28single-precision%29))
  (if (not (Variables|Default|GetHas%20waypoint%20been%20added))
    (bind _asthird_person_character (Utilities|Casting|CastToThirdPersonCharacter (Game|GetPlayerCharacter 0)))
    (bind _output_get (Variables|Default|SetAdded%20Waypoint (Utilities|Struct|MakeWaypoint (Transformation|GetActorTransform _asthird_person_character) (Variables|Default|GetWaypoint%20Color))))
    (Utilities|Array|Add (Variables|/Script/MyProject.Navigation_HUD|Getg_Waypoints (Variables|/Game/ThirdPersonCPP/Blueprints/ThirdPersonCharacter.ThirdPersonCharacter_C|GetNavigation%20HUD _asthird_person_character)) _output_get)
    (Variables|Default|SetHas%20waypoint%20been%20added true)))

(event EventEndPlay
  (params (EndPlayReason :type EEndPlayReason%20Enum :default "Destroyed"))
  (bind _asthird_person_character (Utilities|Casting|CastToThirdPersonCharacter (Game|GetPlayerCharacter 0)))
  (Utilities|Array|RemoveItem (Variables|/Script/MyProject.Navigation_HUD|Getg_Waypoints (Variables|/Game/ThirdPersonCPP/Blueprints/ThirdPersonCharacter.ThirdPersonCharacter_C|GetNavigation%20HUD _asthird_person_character)) (Variables|Default|GetAdded%20Waypoint)))